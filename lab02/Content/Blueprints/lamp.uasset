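; Lamp actor whose spotlight briefly goes dark when a trap fires.
; On BeginPlay it finds the first Trap_dispatcherr in the level and binds its lamp event to that actor's OnTrap dispatcher.
; When triggered, the event prints a debug string, sets the SpotLight intensity to zero, then restores it to a fixed bright value after a short delay.
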(event `self.ReceiveBeginPlay`
  (bind _outactors (`GameplayStatics.GetAllActorsOfClass` "/Game/Blueprints/trap_dispatcherr.trap_dispatcherr_C"))
  (add `/Game/Blueprints/trap_dispatcherr.onTrap` (`|GetArrayItem` _outactors) (delegate `lamp`)))

(event `lamp`
  (`KismetSystemLibrary.PrintString` "lampingggg")
  (`LightComponent.SetIntensity` (`self.SpotLight`) 0.0)
  (`KismetSystemLibrary.Delay` 3.0)
  (`LightComponent.SetIntensity` (`self.SpotLight`) 50000.0))

(fn `UserConstructionScript`)