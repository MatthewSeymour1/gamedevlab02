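; A rotating hazard actor that spins around its local pitch axis while spinning is enabled.
; Tick applies a frame-rate independent rotation by scaling RotationSpeed with delta time when IsSpinning is true.
; BeginPlay enables input from player controller 0, so pressing T calls ToggleSpin to flip IsSpinning.
; The overlap event is empty, so contact with the hazard has no scripted effect.
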(event `self.ReceiveBeginPlay`
  (`self.EnableInput` (`GameplayStatics.GetPlayerController` 0)))

(event `Key|T`
  (params (Key :type "Key Structure"))
  (:`Pressed`
    (`self.ToggleSpin`)))

(event `self.ReceiveTick`
  (params (DeltaSeconds :type "Float (single-precision)"))
  (if (`self.isSpinning`)
    (`self.K2_AddActorLocalRotation` (`KismetMathLibrary.MakeRotator` 0.0 (* DeltaSeconds (`self.rotationSpeed`))))))

(fn `ToggleSpin`
  (set `self.isSpinning` (not (`self.isSpinning`))))

(fn `UserConstructionScript`)